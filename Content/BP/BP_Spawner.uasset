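; BP_Spawner spawns units of a chosen type for its faction.
; SpawnUnit maps a unit ID to one of three unit classes and spawns one, or several when Left Shift is held, at random points in a box around itself.
; Each unit takes the spawner's rotation, has its BPC_Unit component initialized with the faction ID, and is registered with BP_GameState, cached at BeginPlay.
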(event `self.ReceiveBeginPlay`
  (bind _asbp_game_state (cast `/Game/BP/BP_GameState` (`GameplayStatics.GetGameState`)))
  (set `self.As BP Game State` _asbp_game_state))

(fn `SpawnUnit`
  (params (UnitID :type Integer))
  (switch `int` UnitID
    (:`0`
      (set `self.UnitClass` "/Game/BP/BP_Unit00.BP_Unit00_C"))
    (:`1`
      (set `self.UnitClass` "/Game/BP/BP_Unit01.BP_Unit01_C"))
    (:`2`
      (set `self.UnitClass` "/Game/BP/BP_Unit02.BP_Unit02_C")))
  (if (`PlayerController.IsInputKeyDown` (`GameplayStatics.GetPlayerController` 0) "LeftShift")
    (set `self.SpawnQuantity` 5)
    (else
      (set `self.SpawnQuantity` 1)))
  (for _ (range 1 (+ (`self.SpawnQuantity`) 1))
    (bind _returnvalue (`|SpawnActorFromClass` (`self.UnitClass`) (`KismetMathLibrary.Conv_VectorToTransform` (`KismetMathLibrary.RandomPointInBoundingBox` (`self.K2_GetActorLocation`) (800.0 150.0 0.0))) "AdjustIfPossibleButAlwaysSpawn" "OverrideRootScale" null null))
    (`self.K2_SetActorRotation` _returnvalue (`self.K2_GetActorRotation`) false)
    (`/Game/BP/BPC_Unit.Init` (`self.GetComponentByClass` _returnvalue "/Game/BP/BPC_Unit.BPC_Unit_C") (`self.FactionID`))
    (`/Game/BP/BP_GameState.AddUnit` (`self.As BP Game State`) _returnvalue)))

(fn `UserConstructionScript`)