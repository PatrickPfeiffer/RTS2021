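; Unit component for a two-faction battle game, handling faction setup, targeting, attack cooldown, health and death.
; Init spawns and initializes the unit's AI controller, then applies movement speed and red or blue materials.
; FindTarget fetches opposing units from the game state, orders them by repeated minimum-distance picks, and sends the controller toward the first.
; StartAttack only plays muzzle flash and cooldown; TakeDamage updates the health bar and triggers deregistration and destruction at zero.
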(event `Init`
  (params (FactionID :type Integer))
  (bind _returnvalue (select `int` (`self.Faction`) :`0` "/Game/Materials/M_Red.M_Red" :`1` "/Game/Materials/M_Blue.M_Blue" :!type "MaterialInterface Object Reference"))
  (bind _instigator (`Actor.Instigator` (`self.ActorSelf`)))
  (`|ExecutionSequence`
    (:`then_0`
      ;[1 1 1] Set References
      (set `self.ActorSelf` (`self.GetOwner`))
      (bind _asbp_game_state (cast `/Game/BP/BP_GameState` (`GameplayStatics.GetGameState`)))
      (set `self.As BP Game State` _asbp_game_state))
    (:`then_1`
      ;[1 1 1] Spawn Controller
      (`Pawn.SpawnDefaultController` _instigator)
      (bind _asbp_unit_controller (cast `/Game/BP/BP_UnitController` (`Pawn.GetController` _instigator)))
      (bind _output_get (set `self.As BP Unit Controller` _asbp_unit_controller))
      (`/Game/BP/BP_UnitController.Init` _output_get))
    (:`then_2`
      ;[1 1 1] Set Faction & Movement Speed
      (set `self.Faction` FactionID)
      (bind _ascharacter (cast `Character` (`self.ActorSelf`)))
      (set `CharacterMovementComponent.MaxWalkSpeed` (`self.MovementSpeed`) (`Character.CharacterMovement` _ascharacter)))
    (:`then_3`
      ;[1 1 1] Set Material
      (`PrimitiveComponent.SetMaterial` (`self.CharacterMesh`) 0 _returnvalue)
      (`PrimitiveComponent.SetMaterial` (`self.Model`) 0 _returnvalue))))

(event `StartAttack`
  ;[1 1 1] Muzzle Flash & Attack Cooldown
  (set `self.CanAttack` false)
  (`GameplayStatics.SpawnEmitterAttached` (`self.MuzzleFX`) (`self.MuzzlePos`))
  (`KismetSystemLibrary.Delay` (`self.AttackRate`))
  (set `self.CanAttack` true))

(fn `Death`
  (bind _actorself (`self.ActorSelf`))
  (`/Game/BP/BP_GameState.RemoveUnit` (`self.As BP Game State`) _actorself)
  (`Actor.K2_DestroyActor` _actorself))

(fn `FindTarget`
  (bind _unitarray (`/Game/BP/BP_GameState.GetUnitArray` (`self.As BP Game State`) (select `int` (`self.Faction`) :`0` 1 :`1` 0)))
  (switch `int` (`KismetArrayLibrary.Array_Length` _unitarray)
    (:`Default`
      (bind _sortedtargets (`self.Sort Targets` _unitarray))
      (`/Game/BP/BP_UnitController.MoveUnit` (`self.As BP Unit Controller`) (`|GetArrayItem` _sortedtargets)))
    (:`0`
      (return))))

(fn `Sort Targets`
  (params (Targets :type "Array of Actor Object Reference"))
  (returns (SortedTargets :type "Array of Actor Object Reference"))
  (locals (SortedList :type "Array of Actor Object Reference") (TargetActors :type "Array of Actor Object Reference"))
  (bind _sortedlist (`local.SortedList`))
  (bind _distances (`self.Distances`))
  (bind _indexofminvalue (`KismetMathLibrary.MinOfFloatArray` _distances))
  (set `local.TargetActors` Targets)
  (`|ExecutionSequence`
    (:`then_0`
      ;[1 1 1] Clear Arrays
      (`KismetArrayLibrary.Array_Clear` (`self.Distances`))
      (`KismetArrayLibrary.Array_Clear` (`self.NewIndexes`)))
    (:`then_1`
      ;[1 1 1] Get Distance from each potential target
      (for _array_element (`local.TargetActors`)
        (`/Engine/EditorBlueprintResources/StandardMacros.IsValid` _array_element
          (:`Is Valid`
            (`KismetArrayLibrary.Array_Add` (`self.Distances`) (`Actor.GetDistanceTo` (`self.ActorSelf`) _array_element)))))
      ;[1 1 1] Fill New Indexes Array in order of distance
      (`/Engine/EditorBlueprintResources/StandardMacros.ReverseForEachLoop` _distances
        (:`LoopBody`
          (`KismetArrayLibrary.Array_Add` (`self.NewIndexes`) _indexofminvalue)
          (`KismetArrayLibrary.Array_Remove` (`self.Distances`) _indexofminvalue))
        (:`Completed`
          ;[1 1 1] Return sorted list of targets by distance
          (for _array_element_2 (`self.NewIndexes`)
            (`KismetArrayLibrary.Array_Add` _sortedlist (`|GetArrayItem` (`local.TargetActors`) _array_element_2)))
          (return _sortedlist))))))

(fn `TakeDamage`
  (params (Damge :type Integer))
  (returns (IsDead :type Boolean))
  ;[1 1 1] Remove Health
  (bind _output_get (set `self.Health` (- (`self.Health`) Damge)))
  ;[1 1 1] Get HealthBar ref
  (bind _asw_health_bar (cast `/Game/BP/Widgets/W_HealthBar` (`WidgetComponent.GetWidget` (`self.W_HealthBar`))))
  (`/Game/BP/Widgets/W_HealthBar.SetHealthBar` _asw_health_bar (/ (`KismetMathLibrary.Conv_IntToDouble` (`self.Health`)) (`KismetMathLibrary.Conv_IntToDouble` (`self.MaxHealth`))))
  (if (<= _output_get 0)
    (`self.Death`)
    (return true)
    (else
      (return false))))