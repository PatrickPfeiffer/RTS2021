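; Game state for a two-faction unit battle that tracks each side's units and whether combat is active.
; It caches all BP_Spawner actors at BeginPlay and forwards spawn requests to those matching the requested faction.
; Units are sorted into per-faction arrays by their BPC_Unit component, which StartAttack tells to find targets.
; Removing units ends combat when either side is empty, and RemoveAllUnits kills every unit, iterating in reverse.
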(event `self.ReceiveBeginPlay`
  (bind _outactors (`GameplayStatics.GetAllActorsOfClass` "/Game/BP/BP_Spawner.BP_Spawner_C"))
  (set `self.Spawners` _outactors))

(event `AddUnit`
  (params (NewUnit :type "Actor Object Reference"))
  (switch `int` (`/Game/BP/BPC_Unit.Faction` (`self.GetComponentByClass` NewUnit "/Game/BP/BPC_Unit.BPC_Unit_C"))
    (:`0`
      (`KismetArrayLibrary.Array_Add` (`self.UnitsFaction0`) NewUnit))
    (:`1`
      (`KismetArrayLibrary.Array_Add` (`self.UnitsFaction1`) NewUnit))))

(fn `GetUnitArray`
  (params (FactionID :type Integer))
  (returns (UnitArray :type "Array of Actor Object Reference"))
  (switch `int` FactionID
    (:`0`
      (return (`self.UnitsFaction0`)))
    (:`1`
      (return (`self.UnitsFaction1`)))))

(fn `RemoveAllUnits`
  (bind (_arrayindex _arrayelement) (`/Engine/EditorBlueprintResources/StandardMacros.ReverseForEachLoop` (`self.UnitsFaction0`))
    (:`LoopBody`
      (`/Game/BP/BPC_Unit.Death` (`self.GetComponentByClass` _arrayelement "/Game/BP/BPC_Unit.BPC_Unit_C")))
    (:`Completed`
      (bind (_arrayindex_2 _arrayelement_2) (`/Engine/EditorBlueprintResources/StandardMacros.ReverseForEachLoop` (`self.UnitsFaction1`))
        (:`LoopBody`
          (`/Game/BP/BPC_Unit.Death` (`self.GetComponentByClass` _arrayelement_2 "/Game/BP/BPC_Unit.BPC_Unit_C")))))))

(fn `RemoveUnit`
  (params (Unit :type "Actor Object Reference"))
  (`KismetArrayLibrary.Array_RemoveItem` (select `int` (`/Game/BP/BPC_Unit.Faction` (`self.GetComponentByClass` Unit "/Game/BP/BPC_Unit.BPC_Unit_C")) :`0` (`self.UnitsFaction0`) :`1` (`self.UnitsFaction1`)) Unit)
  (`|ExecutionSequence`
    (:`then_0`
      (if (== (`KismetArrayLibrary.Array_Length` (`self.UnitsFaction0`)) 0)
        (set `self.CombatActive` false :!label _label)))
    (:`then_1`
      (if (== (`KismetArrayLibrary.Array_Length` (`self.UnitsFaction1`)) 0)
        (goto _label)))))

(fn `SpawnUnit`
  (params (Faction :type Integer) (UnitID :type Integer))
  (for (_array_element _array_index) (`self.Spawners`)
    (if (== Faction (`/Game/BP/BP_Spawner.FactionID` _array_element))
      (`/Game/BP/BP_Spawner.SpawnUnit` (`|GetArrayItem` (`self.Spawners`) _array_index) UnitID))))

(fn `StartAttack`
  (set `self.CombatActive` true)
  (for _array_element (`self.UnitsFaction0`)
    (`/Game/BP/BPC_Unit.FindTarget` (`self.GetComponentByClass` _array_element "/Game/BP/BPC_Unit.BPC_Unit_C")))
  (for _array_element_2 (`self.UnitsFaction1`)
    (`/Game/BP/BPC_Unit.FindTarget` (`self.GetComponentByClass` _array_element_2 "/Game/BP/BPC_Unit.BPC_Unit_C"))))

(fn `UserConstructionScript`)