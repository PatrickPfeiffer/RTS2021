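; BP_Unit00 is a unit Blueprint that delegates to its BPCUnit component.
; On BeginPlay it passes its health bar widget component, skeletal mesh, Model and MuzzlePos references to BPCUnit.
; It then casts the health bar's widget to W_HealthBar and calls ChangeSize on it.
; The construction script is empty.
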(event `self.ReceiveBeginPlay`
  (bind _bpc_unit (`self.BPC_Unit`))
  (set `/Game/BP/BPC_Unit.W_HealthBar` (`self.W_HealthBar`) _bpc_unit)
  (set `/Game/BP/BPC_Unit.CharacterMesh` (`self.SkeletalMesh`) _bpc_unit)
  (set `/Game/BP/BPC_Unit.Model` (`self.Model`) _bpc_unit)
  (set `/Game/BP/BPC_Unit.MuzzlePos` (`self.MuzzlePos`) _bpc_unit)
  (bind _asw_health_bar (cast `/Game/BP/Widgets/W_HealthBar` (`WidgetComponent.GetWidget` (`self.W_HealthBar`))))
  (`/Game/BP/Widgets/W_HealthBar.ChangeSize` _asw_health_bar))

(fn `UserConstructionScript`)