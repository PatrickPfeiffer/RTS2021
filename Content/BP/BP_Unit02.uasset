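; BP_Unit02 is a unit Blueprint that delegates to a BPCUnit component and adds a continuously spinning model part.
; On BeginPlay it hands BPCUnit its health bar widget, skeletal mesh, model and muzzle position references.
; Each Tick it yaws Model1 at a constant, frame-rate-independent speed.
; The construction script is empty.
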(event `self.ReceiveBeginPlay`
  (bind _bpc_unit (`self.BPC_Unit`))
  (set `/Game/BP/BPC_Unit.W_HealthBar` (`self.W_HealthBar`) _bpc_unit)
  (set `/Game/BP/BPC_Unit.CharacterMesh` (`self.SkeletalMesh`) _bpc_unit)
  (set `/Game/BP/BPC_Unit.Model` (`self.Model`) _bpc_unit)
  (set `/Game/BP/BPC_Unit.MuzzlePos` (`self.MuzzlePos`) _bpc_unit))

(event `self.ReceiveTick`
  (params (DeltaSeconds :type "Float (single-precision)"))
  (`SceneComponent.K2_AddRelativeRotation` (`self.Model1`) (`KismetMathLibrary.MakeRotator` 0.0 0.0 (* DeltaSeconds 500.0)) false false))

(fn `UserConstructionScript`)