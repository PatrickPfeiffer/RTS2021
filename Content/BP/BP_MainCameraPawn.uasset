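; BP_MainCameraPawn is a top-down-style camera pawn with mouse edge scrolling and zoom, which also adds the W_MainOverlay widget to the viewport on BeginPlay.
; The Zoom axis changes the Boom arm length, scaled by frame time and ZoomSpeed and clamped between minimum and maximum distances.
; Each Tick, MouseMoveOnAxis runs per screen axis, adding world-space movement input when the cursor is within ScreenEdge of a viewport border.
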(event `self.ReceiveBeginPlay`
  (bind _returnvalue (`|CreateWidget` "/Game/BP/Widgets/W_MainOverlay.W_MainOverlay_C"))
  (`UserWidget.AddToViewport` _returnvalue 0))

(event `InputAxis|Zoom`
  (params (AxisValue :type "Float (single-precision)"))
  (bind _boom (`self.Boom`))
  (set `SpringArmComponent.TargetArmLength` (`KismetMathLibrary.FClamp` (+ (`SpringArmComponent.TargetArmLength` _boom) (* (* AxisValue -1.0) (* (`GameplayStatics.GetWorldDeltaSeconds`) (`self.ZoomSpeed`)))) (`self.MinCamDistance`) (`self.MaxCamDistance`)) _boom))

(event `self.ReceiveTick`
  (params (DeltaSeconds :type "Float (single-precision)"))
  (bind (_returnvalue_x _returnvalue_y) (`KismetMathLibrary.BreakVector2D` (`WidgetLayoutLibrary.GetViewportSize`)))
  (bind (_locationx _locationy) (`PlayerController.GetMousePosition` (`GameplayStatics.GetPlayerController` 0)))
  (`WidgetLayoutLibrary.GetMousePositionOnViewport`)
  (`self.MouseMoveOnAxis` _locationx _returnvalue_x (0.0 -1.0 0.0))
  (`self.MouseMoveOnAxis` _locationy _returnvalue_y (1.0 0.0 0.0)))

(fn `MouseMoveOnAxis`
  (params (MousePos :type "Float (double-precision)") (ScreenSize :type "Float (double-precision)") (Axis :type "Vector Structure"))
  (bind _returnvalue (- ScreenSize MousePos))
  (if (< _returnvalue (`self.ScreenEdge`))
    (`self.AddMovementInput` Axis -1.0)
    (elif (> _returnvalue (- ScreenSize (`self.ScreenEdge`)))
      (`self.AddMovementInput` Axis))))

(fn `UserConstructionScript`)